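; BP_MerchantPlayer is the player Blueprint for the merchant, managing which Sphera items are selected and their combined score.
; BeginPlay creates the merchant and skin percent information widgets, plus a tutorial widget if the GameInstance's MerchantTutorial flag is false.
; AddObjectSelected fills the first empty slot in ObjectsSelected, rejecting duplicates by ItemReference, while RemoveObject clears the matching slot.
; Both adjust the running score from the item's DA_Sphera data and refresh the merchant screen.
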(event `self.ReceiveBeginPlay`
  (bind _returnvalue (`|CreateWidget` "/Game/UI/Merchant/WBP_Merchant.WBP_Merchant_C"))
  (`UserWidget.AddToViewport` _returnvalue 0)
  (set `self.WBP_Merchant` _returnvalue)
  (bind _returnvalue_2 (`|CreateWidget` "/Game/UI/Merchant/WBP_SkinPercentInformation.WBP_SkinPercentInformation_C"))
  (`UserWidget.AddToViewport` _returnvalue_2 0)
  (set `self.WBP_SkinInformation` _returnvalue_2)
  (if (not (`/Game/Blueprint/BP_GameInstance.merchantTutorial` (`/Game/Blueprint/FL_MainFunctionLibrary.GetGameInstanceBP`)))
    (bind _returnvalue_3 (`|CreateWidget` "/Game/UI/Tutorial/WBP_MerchantTuto.WBP_MerchantTuto_C"))
    (`UserWidget.AddToViewport` _returnvalue_3 0)))

(fn `AddObjectSelected`
  (params (NewItem :type "/Game/UI/WBP_SlotsObject Object Reference (by ref)"))
  (bind _objectsselected (`self.ObjectsSelected`))
  (bind _newitem (`local.NewItem`))
  ;[1 1 1] Check if not already selected
  (for _array_element (`self.ObjectsSelected`)
    (`/Engine/EditorBlueprintResources/StandardMacros.IsValid` _array_element
      (:`Is Valid`
        (if (== (`/Game/UI/WBP_SlotsObject.itemReference` _array_element) (`/Game/UI/WBP_SlotsObject.itemReference` NewItem))
          (return)))))
  (for (_array_element_2 _array_index) _objectsselected
    (`/Engine/EditorBlueprintResources/StandardMacros.IsValid` _array_element_2
      (:`Is Not Valid`
        (`KismetArrayLibrary.Array_Set` _objectsselected _array_index _newitem)
        (set `self.additiveScoreSphera` (+ (`self.additiveScoreSphera`) (`/Game/ItemData/DA_Sphera.Score` (cast `/Game/ItemData/DA_Sphera` (`/Game/UI/WBP_SlotsObject.itemReference` _newitem) :!pure true))))
        (`/Game/UI/Merchant/WBP_Merchant.RefreshScreen` (`self.WBP_Merchant`))
        (return)))))

(fn `RemoveObject`
  (params (ItemToRemove :type "/Game/UI/WBP_SlotsObject Object Reference (by ref)"))
  (bind _objectsselected (`self.ObjectsSelected`))
  (for (_array_element _array_index) _objectsselected
    (`/Engine/EditorBlueprintResources/StandardMacros.IsValid` _array_element
      (:`Is Valid`
        (if (== (`/Game/UI/WBP_SlotsObject.itemReference` _array_element) (`/Game/UI/WBP_SlotsObject.itemReference` ItemToRemove))
          (`KismetArrayLibrary.Array_Set` _objectsselected _array_index)
          (set `self.additiveScoreSphera` (- (`self.additiveScoreSphera`) (`/Game/ItemData/DA_Sphera.Score` (cast `/Game/ItemData/DA_Sphera` (`/Game/UI/WBP_SlotsObject.itemReference` ItemToRemove) :!pure true))))
          (`/Game/UI/Merchant/WBP_Merchant.RefreshScreen` (`self.WBP_Merchant`))
          (return))))))

(fn `UserConstructionScript`)