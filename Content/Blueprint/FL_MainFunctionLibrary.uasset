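; Blueprint function library of shared inventory, skin and save helpers, most of which route through BP_GameInstance.
; Builds inventory slot widgets for a given class in rows of six, showing Score for DA_Sphera items and amount for others, with a selling-mode flag.
; Filters owned skins by rarity, and draws a shuffled random set from stored skin pools using a count per rarity, with duplicates possible.
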(fn `CreateWidgetsSlotInWidget`
  (params (`Widget to create in` :type "PanelWidget Object Reference") (Class :type "/Game/ItemData/DA_BaseInventoryObject Class Reference") (`SellingMode?` :type Boolean))
  (locals (CurrentHorizontalBox :type "/Game/UI/WBP_HorizontalBoxContainers Object Reference"))
  (for (_array_element _array_index) (`/Game/Blueprint/BP_GameInstance.GetAllActorOfClassInInventory` (cast `/Game/Blueprint/BP_GameInstance` (`GameplayStatics.GetGameInstance` null) :!pure true) Class)
    (if (== (mod _array_index 6) 0)
      ;[1 1 1] CreateNewHorizontal box each 6 slot
      (bind _returnvalue (`|CreateWidget` "/Game/UI/WBP_HorizontalBoxContainers.WBP_HorizontalBoxContainers_C"))
      (set `local.CurrentHorizontalBox` _returnvalue)
      (`PanelWidget.AddChild` (`local.Widget to create in`) _returnvalue))
    (bind _returnvalue_2 (`|CreateWidget` "/Game/UI/WBP_SlotsObject.WBP_SlotsObject_C" null (`local.SellingMode?`)))
    (`/Game/UI/WBP_SlotsObject.SetItemReference` _returnvalue_2 _array_element)
    (bind _asda_sphera (cast `/Game/ItemData/DA_Sphera` _array_element)
      (:`then`
        (bind _image (`/Game/ItemData/DA_BaseInventoryObject.GetImage` _array_element))
        (`/Game/UI/WBP_SlotsObject.ChangeImageAndText` _returnvalue_2 (`/Game/ItemData/DA_Sphera.Score` _asda_sphera) _image))
      (:`CastFailed`
        (`/Game/UI/WBP_SlotsObject.ChangeImageAndText` _returnvalue_2 (`/Game/ItemData/DA_BaseInventoryObject.GetAmount` _array_element) _image)))
    (`UserWidget.SetPadding` _returnvalue_2 (make `Margin` 15.0 15.0 15.0 15.0))
    (`HorizontalBox.AddChildToHorizontalBox` (`/Game/UI/WBP_HorizontalBoxContainers.HorizontalBox_33` (`local.CurrentHorizontalBox`)) _returnvalue_2)))

(fn `Get Random Skin Per Rarity`
  (params (Common :type Integer) (Uncommon :type Integer) (Rare :type Integer) (Epic :type Integer) (Legendary :type Integer) (Mythic :type Integer))
  (returns (Skin :type "Array of /Game/ItemData/Skin/DA_Skin Object Reference"))
  (locals (tmpSkin :type "Array of /Game/ItemData/Skin/DA_Skin Object Reference") (tmpSkinAmount :type Integer) (Index :type Integer))
  (bind _tmpskin (`local.tmpSkin`))
  (set `local.tmpSkinAmount` Common)
  (for _index (range 6)
    (for _ (range (`local.tmpSkinAmount`))
      (bind _skin (`/Game/Blueprint/BP_GameInstance.GetSkinStoredByRarity` (`self.GetGameInstanceBP` null) (cast `/Game/Miscellaneous/Enum_Rarity` (`KismetMathLibrary.Conv_IntToByte` _index))))
      (`KismetArrayLibrary.Array_Add` (`local.tmpSkin`) (`|GetArrayItem` _skin (`KismetMathLibrary.RandomInteger` (- (`KismetArrayLibrary.Array_Length` _skin) 1)))))
    (bind _output_get (set `local.Index` (+ (`local.Index`) 1)))
    (switch `int` _output_get
      (:`1`
        (set `local.tmpSkinAmount` (`local.Uncommon`)))
      (:`2`
        (set `local.tmpSkinAmount` (`local.Rare`)))
      (:`3`
        (set `local.tmpSkinAmount` (`local.Epic`)))
      (:`4`
        (set `local.tmpSkinAmount` (`local.Legendary`)))
      (:`5`
        (set `local.tmpSkinAmount` (`local.Mythic`)))))
  (`KismetArrayLibrary.Array_Shuffle` _tmpskin)
  (return _tmpskin))

(fn `GetAllActorOfClassInInventory`
  (params (ObjectType :type "/Game/ItemData/DA_BaseInventoryObject Class Reference"))
  (returns (List :type "Array of /Game/ItemData/DA_BaseInventoryObject Object Reference"))
  (return (`/Game/Blueprint/BP_GameInstance.GetAllActorOfClassInInventory` (`self.GetGameInstanceBP` null) ObjectType)))

(fn `GetAllSkinOfRarity`
  (params (Rarity :type "/Game/Miscellaneous/Enum_Rarity Enum" :default "NewEnumerator0"))
  (returns (List :type "Array of /Game/ItemData/Skin/DA_Skin Object Reference"))
  (locals (Items :type "Array of /Game/ItemData/Skin/DA_Skin Object Reference"))
  (for _array_element (`self.GetAllActorOfClassInInventory` "/Game/ItemData/Skin/DA_Skin.DA_Skin_C")
    (bind _asda_skin (cast `/Game/ItemData/Skin/DA_Skin` _array_element))
    (if (`|EnumEquality` (`/Game/ItemData/DA_BaseInventoryObject.GetRarity` _asda_skin) (`local.Rarity`))
      (`KismetArrayLibrary.Array_Add` (`local.Items`) _asda_skin)))
  (return (`local.Items`)))

(fn `GetGameInstanceBP`
  (returns (`AsBP Game Instance` :type "/Game/Blueprint/BP_GameInstance Object Reference"))
  (return (cast `/Game/Blueprint/BP_GameInstance` (`GameplayStatics.GetGameInstance` null) :!pure true)))

(fn `SaveGame`
  (`/Game/Blueprint/BP_GameInstance.SaveGame` (`self.GetGameInstanceBP` null)))