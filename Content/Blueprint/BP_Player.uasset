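; Player pawn for a one-touch swinging game: taps attach it to overlapped attach points to orbit on a rope, or fling it off tangentially.
; Tick drives orbits from precomputed GameInstance circle tables; detached flight uses physics.
; Attaching scores by rope length and a height-above-dead-zone multiplier; falling below that zone or leaving attach-point range triggers death.
; Also manages UI widgets, respawn, parallax clouds and a time-dilation tutorial.
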(event `TimeDilatationTimelinePlay`
  (bind (_direction _timedilatation) (`Timeline|DecreaseTimeDilatation` :`NewTime` (stale `TimeDilatationTimelineSetNewTime` time) :!label _label)
    (:`Update`
      (`GameplayStatics.SetGlobalTimeDilation` _timedilatation))
    (:`Finished`
      (bind _returnvalue (< _timedilatation 0.1))
      (if _returnvalue
        (`/Game/UI/Tutorial/WBP_TextHowTOPlay.ShowScreen` (`self.WBP_TextHowToPlay`) (`self.HowToPlayTutorialInt`))
        (`GameplayStatics.SetGlobalTimeDilation` 0.0001))
      (`KismetSystemLibrary.Delay` (`KismetMathLibrary.SelectFloat` 0.0006 1.0 _returnvalue))
      (set `self.CanClickHowToPlayTutorial` true))))

(event `TimeDilatationTimelineReverse`
  (goto _label :!via `Reverse`))

(event `TimeDilatationTimelineSetNewTime`
  (params (time :type "Float (double-precision)"))
  (goto _label :!via `SetNewTime`))

(event `TouchHowToPlayTutorial`
  (bind _howtoplaytutorialint (`self.HowToPlayTutorialInt`))
  (bind _returnvalue (<= _howtoplaytutorialint 7))
  ;[1 1 1] TutorialHowToPlay
  (if (`self.CanClickHowToPlayTutorial`)
    (`/Game/UI/Tutorial/WBP_TextHowTOPlay.HideScreen` (`self.WBP_TextHowToPlay`))
    (if (`self.isAttached?`)
      (`self.DettachPlayer`)
      (if _returnvalue
        (`/Engine/EditorBlueprintResources/StandardMacros.IncrementInt` _howtoplaytutorialint
          (:`  `
            (if (<= (`self.HowToPlayTutorialInt`) 6)
              (set `self.CanClickHowToPlayTutorial` false)
              (`|ExecutionSequence`
                (:`then_0`
                  (`self.TimeDilatationTimelineSetNewTime` 0.7))
                (:`then_1`
                  (`self.TimeDilatationTimelineReverse`)
                  (`KismetSystemLibrary.Delay` 0.2)
                  (`self.TimeDilatationTimelinePlay`)
                  (set `self.timeToWaitTutorialHowToPlay` 1.8)))))))
      (else
        (`self.Attach Player`)
        (if _returnvalue
          (`/Engine/EditorBlueprintResources/StandardMacros.IncrementInt` _howtoplaytutorialint
            (:`  `
              (set `self.CanClickHowToPlayTutorial` false)
              (if (not (`/Game/Blueprint/BP_GameInstance.DidHowToPlayTutorial` (`/Game/Blueprint/FL_MainFunctionLibrary.GetGameInstanceBP`)))
                (`|ExecutionSequence`
                  (:`then_0`
                    (`self.TimeDilatationTimelineSetNewTime` 0.7))
                  (:`then_1`
                    (`self.TimeDilatationTimelineReverse`)
                    (if (<= (`self.HowToPlayTutorialInt`) 6)
                      (`KismetSystemLibrary.Delay` (`self.timeToWaitTutorialHowToPlay`))
                      (`self.TimeDilatationTimelinePlay`))))))))))))

(event `DettachPlayer`
  (bind _indexcurrentangle (`self.IndexCurrentAngle`))
  (bind _mesh (`self.Mesh`))
  (bind _returnvalue (`KismetMathLibrary.VSize` (`self.vectoAttachActor`)))
  (bind _returnvalue_2 (+ _indexcurrentangle 1))
  (bind _ycoordinatecircle (`/Game/Blueprint/BP_GameInstance.YCoordinateCircle` (`self.GameInstance`)))
  (bind _zcoordinatecircle (`/Game/Blueprint/BP_GameInstance.ZCoordinateCircle` (`self.GameInstance`)))
  (bind (_x _y _z) (`KismetMathLibrary.BreakVector3f` (`self.K2_GetActorLocation` (`self.overlappedAttachPoint`))))
  (bind _returnvalue_3 (`KismetMathLibrary.SelectInt` 0 _returnvalue_2 (> _returnvalue_2 (`KismetArrayLibrary.Array_Length` (`/Game/Blueprint/BP_GameInstance.YCoordinateCircle` (`self.GameInstance`))))))
  (bind _returnvalue_4 (* (`KismetMathLibrary.Normal` (- (`KismetMathLibrary.MakeVector` 0.0 (+ _y (* _returnvalue (`|GetArrayItem` _ycoordinatecircle _returnvalue_3))) (+ _z (* (`|GetArrayItem` _zcoordinatecircle _returnvalue_3) _returnvalue))) (`KismetMathLibrary.MakeVector` 0.0 (+ _y (* _returnvalue (`|GetArrayItem` _ycoordinatecircle _indexcurrentangle))) (+ _z (* (`|GetArrayItem` _zcoordinatecircle _indexcurrentangle) _returnvalue))))) (* (`KismetMathLibrary.FFloor` (`self.speed`)) 10)))
  (set `self.isAttached?` false)
  (`PrimitiveComponent.SetSimulatePhysics` _mesh true)
  (`PrimitiveComponent.SetPhysicsLinearVelocity` _mesh (0.0 0.0 0.0) false "None")
  (`PrimitiveComponent.SetPhysicsLinearVelocity` _mesh (`KismetMathLibrary.SelectVector` _returnvalue_4 (`KismetMathLibrary.NegateVector` _returnvalue_4) (`self.rotateClockwise?`)) false "None")
  (`SceneComponent.SetHiddenInGame` (`self.Rope`) true false))

(event `Play`
  (if (`self.firstTouch?`)
    (`self.FirstTouch`)
    (`/Game/Blueprint/GameManager/BP_GameManagerMaster.StartGame` (`self.GameManager`))
    (if (not (`/Game/Blueprint/BP_GameInstance.DidHowToPlayTutorial` (`/Game/Blueprint/FL_MainFunctionLibrary.GetGameInstanceBP`)))
      (`self.TimeDilatationTimelinePlay`)
      (bind _returnvalue (`|CreateWidget` "/Game/UI/Tutorial/WBP_TextHowTOPlay.WBP_TextHowTOPlay_C"))
      (`UserWidget.AddToViewport` _returnvalue 0)
      (set `self.WBP_TextHowToPlay` _returnvalue))))

(event `self.ReceiveBeginPlay`
  (bind _returnvalue (`GameplayStatics.GetPlayerController` 0))
  ;[1 0.9242 0.9115] FirstTouch/BeginPlay
  (`|ExecutionSequence`
    (:`then_0`
      (`|ExecutionSequence`
        (:`then_0`
          (bind _output_get (set `self.GameInstance` (cast `/Game/Blueprint/BP_GameInstance` (`GameplayStatics.GetGameInstance`) :!pure true)))
          (if (!= (`/Game/Blueprint/BP_GameInstance.CurrentEquippedSkin` _output_get) null)
            (bind _skeletalmesh (`/Game/ItemData/Skin/DA_Skin.GetSkeletalMesh` (`/Game/Blueprint/BP_GameInstance.GetCurrentEquippedSkin` _output_get)))
            (`SkinnedMeshComponent.SetSkinnedAssetAndUpdate` (`self.Skin`) _skeletalmesh false)
            (else
              (`/Game/Blueprint/BP_GameInstance.SetCurrentEquippedSkin` _output_get "/Game/ItemData/Skin/DA_Skin_Shuriken.DA_Skin_Shuriken_C"))))
        (:`then_1`
          (`/Game/Blueprint/BP_GameInstance.BeginPlay` (`self.GameInstance`))
          (`/Game/Blueprint/BP_PlayerController.PossessEntity` (cast `/Game/Blueprint/BP_PlayerController` (`GameplayStatics.GetPlayerController` 0) :!pure true) self)
          (`WidgetLayoutLibrary.RemoveAllWidgets`)
          (bind _returnvalue_2 (`|CreateWidget` "/Game/UI/WBP_MainMenu.WBP_MainMenu_C" _returnvalue))
          (`UserWidget.AddToViewport` _returnvalue_2 0)
          (set `self.WBP_MainMenu` _returnvalue_2)
          (set `PlayerController.bShowMouseCursor` true _returnvalue))))
    (:`then_1`
      (bind _returnvalue_3 (`|CreateWidget` "/Game/UI/WBP_DeathScreen.WBP_DeathScreen_C" _returnvalue))
      (`UserWidget.AddToViewport` _returnvalue_3 0)
      (set `self.WBP_DeathScreen` _returnvalue_3)
      (`self.CreateDynamicBackgroundParalax`))
    (:`then_2`
      (bind _returnvalue_4 (`|CreateWidget` "/Game/UI/WBP_GameMenu.WBP_GameMenu_C"))
      (`UserWidget.AddToViewport` _returnvalue_4 0)
      (set `self.WBP_GameMenu` _returnvalue_4)
      (bind _returnvalue_5 (`|CreateWidget` "/Game/UI/Chest/WBP_OpenChest.WBP_OpenChest_C" (`GameplayStatics.GetPlayerController` 0)))
      (`UserWidget.AddToViewport` _returnvalue_5 0)
      (set `self.WBP_OpenChest` _returnvalue_5))
    (:`then_3`
      (set `/Game/Blueprint/BP_GameInstance.PlayerPawn` self (`self.GameInstance`))
      (bind _returnvalue_6 (`|CreateWidget` "/Game/UI/Chest/WBP_ChestInventoryScreen.WBP_ChestInventoryScreen_C" (`GameplayStatics.GetPlayerController` 0)))
      (`UserWidget.AddToViewport` _returnvalue_6 0)
      (set `self.WBP_ChangeChestScreen` _returnvalue_6)
      (`KismetSystemLibrary.Delay` 0.01)
      (`/Game/UI/WBP_MainMenu.RefreshScreen` (`self.WBP_MainMenu`))
      (set `self.speed` (`self.baseSpeed`)))))

(event `InputTouch`
  (params (Location :type "Vector Structure") (FingerIndex :type "ETouchIndex Enum"))
  (:`Pressed`
    (if (`self.firstTouch?`) :!label _label_2
      _
      (elif (`/Game/Blueprint/BP_GameInstance.DidHowToPlayTutorial` (`/Game/Blueprint/FL_MainFunctionLibrary.GetGameInstanceBP`))
        (if (`self.isAttached?`)
          (`self.DettachPlayer`)
          (else
            (`self.Attach Player`)))
        (else
          (`self.TouchHowToPlayTutorial`))))))

(event `Key|LeftMouseButton`
  (params (Key :type "Key Structure"))
  (:`Pressed`
    (goto _label_2)))

(event `Attach Player`
  (bind _mesh (`self.Mesh`))
  (bind _returnvalue (- (`SceneComponent.K2_GetComponentLocation` _mesh) (`self.K2_GetActorLocation` (`self.overlappedAttachPoint`))))
  (bind _returnvalue_2 (`KismetMathLibrary.Normal` _returnvalue))
  (bind _returnvalue_3 (`KismetMathLibrary.DegAcos` (`KismetMathLibrary.Dot_VectorVector` _returnvalue_2 (`SceneComponent.GetRightVector` _mesh))))
  (`/Engine/EditorBlueprintResources/StandardMacros.IsValid` (`self.overlappedAttachPoint`)
    (:`Is Valid`
      (set `self.isAttached?` true)
      (set `self.vectoAttachActor` _returnvalue)
      (`SceneComponent.SetHiddenInGame` (`self.Rope`) false false)
      (set `self.rotateClockwise?` (> (`KismetMathLibrary.BreakVector3f` (`KismetMathLibrary.Cross_VectorVector` (`KismetMathLibrary.Normal` (`self.vectoAttachActor`)) (`KismetMathLibrary.Normal` (`SceneComponent.GetComponentVelocity` (`self.Mesh`))))) 0.0))
      (set `self.IndexCurrentAngle` (`KismetMathLibrary.FFloor` (* (`KismetMathLibrary.SelectFloat` _returnvalue_3 (+ 180.0 (`KismetMathLibrary.Abs` (- _returnvalue_3 180.0))) (> (`.Z` (`KismetMathLibrary.BreakVector3f` _returnvalue_2)) 0.0)) (/ (`KismetArrayLibrary.Array_Length` (`/Game/Blueprint/BP_GameInstance.YCoordinateCircle` (`self.GameInstance`))) 360))))
      (`PrimitiveComponent.SetSimulatePhysics` (`self.Mesh`) false)
      (`self.AddScore` (* (`self.BaseAddAmountScore`) (/ (`KismetMathLibrary.VSize` (`self.vectoAttachActor`)) 425.0))))))

(event `FirstTouch`
  ;[1 0.9242 0.9115] FirstTouch/BeginPlay
  (`PrimitiveComponent.SetSimulatePhysics` (`self.Mesh`) true)
  (set `self.firstTouch?` false)
  (`/Game/UI/WBP_MainMenu.HidePressToPlay` (`self.WBP_MainMenu`))
  (`/Game/UI/WBP_GameMenu.Show_HideGameMenu` (`self.WBP_GameMenu`) true))

(event `self.Mesh.OnComponentBeginOverlap`
  (params (OverlappedComponent :type "PrimitiveComponent Object Reference") (OtherActor :type "Actor Object Reference") (OtherComp :type "PrimitiveComponent Object Reference") (OtherBodyIndex :type Integer) (bFromSweep :type Boolean) (SweepResult :type "HitResult Structure (by ref)"))
  ;[1 1 1] Overlap system
  (if (`self.isAttached?`)
    _
    (elif (== (`GameplayStatics.GetObjectClass` OtherActor) "/Game/Blueprint/BP_AttachPoint.BP_AttachPoint_C")
      (bind _asbp_attach_point (cast `/Game/Blueprint/BP_AttachPoint` OtherActor))
      (set `self.overlappedAttachPoint` _asbp_attach_point))))

(event `Death`
  ;[1 1 1] Death
  (if (not (`self.isDead`))
    (set `self.isDead` true)
    (if (`self.isAttached?`)
      (`self.DettachPlayer`))
    (`/Game/UI/WBP_DeathScreen.SetScoreValue` (`self.WBP_DeathScreen`) (`self.currentScore`))
    (`SceneComponent.K2_AttachToComponent` (`self.Camera`) (`self.Root`) "None" "KeepWorld" "KeepWorld" "KeepWorld" false)
    (`SceneComponent.K2_AttachToComponent` (`self.background`) (`self.Root`) "None" "KeepWorld" "KeepWorld" "KeepWorld" false)
    (`|ExecutionSequence`
      (:`then_0`
        (`/Game/UI/WBP_DeathScreen.FadeInAll` (`self.WBP_DeathScreen`))
        (`/Game/UI/WBP_GameMenu.Show_HideGameMenu` (`self.WBP_GameMenu`) false)
        (`/Game/Blueprint/BP_DeadZone.EndGame` (`/Game/Blueprint/GameManager/BP_GameManagerMaster.DeadZone` (`self.GameManager`)))
        (if (`self.CanClickHowToPlayTutorial`)
          (`KismetSystemLibrary.Delay` 0.5)
          (bind _returnvalue (`|CreateWidget` "/Game/UI/Tutorial/WBP_EndGameTuto.WBP_EndGameTuto_C"))
          (`UserWidget.AddToViewport` _returnvalue 0)))
      (:`then_1`
        (`KismetSystemLibrary.Delay` 2.0)
        (if (`self.isDead`)
          (`PrimitiveComponent.SetSimulatePhysics` (`self.Mesh`) false))))))

(event `self.Mesh.OnComponentEndOverlap`
  (params (OverlappedComponent :type "PrimitiveComponent Object Reference") (OtherActor :type "Actor Object Reference") (OtherComp :type "PrimitiveComponent Object Reference") (OtherBodyIndex :type Integer))
  (bind _overlappedattachpoint (`self.overlappedAttachPoint`))
  ;[1 1 1] Overlap system
  (`/Engine/EditorBlueprintResources/StandardMacros.IsValid` _overlappedattachpoint
    (:`Is Valid`
      (if (== OtherActor _overlappedattachpoint)
        (set `self.overlappedAttachPoint` null)))))

(event `self.Sphere.OnComponentEndOverlap`
  (params (OverlappedComponent :type "PrimitiveComponent Object Reference") (OtherActor :type "Actor Object Reference") (OtherComp :type "PrimitiveComponent Object Reference") (OtherBodyIndex :type Integer))
  ;[1 1 1] Overlap system
  (if (`KismetArrayLibrary.Array_IsEmpty` (`PrimitiveComponent.GetOverlappingActors` (`self.Sphere`) "/Game/Blueprint/BP_AttachPoint.BP_AttachPoint_C"))
    (`self.Death`)))

(event `Respawn`
  (bind _wbp_gamemenu (`self.WBP_GameMenu`))
  (bind _returnvalue (`KismetMathLibrary.FFloor` (`self.currentScore`)))
  ;[1 1 1] Respawn
  (if (!= _returnvalue 0)
    (`/Game/Blueprint/BP_GameInstance.AddBallToInventory` (`self.GameInstance`) (`/Game/Blueprint/BP_GameInstance.GetCurrentEquippedSkin` (`/Game/Blueprint/FL_MainFunctionLibrary.GetGameInstanceBP`)) _returnvalue))
  (`/Game/Blueprint/GameManager/BP_GameManagerMaster.RestartGame` (`self.GameManager`))
  (`/Game/UI/WBP_DeathScreen.ResetRenderOpacity` (`self.WBP_DeathScreen`))
  (`self.ResetPlayer`)
  (`/Game/UI/WBP_MainMenu.ShowPressToPlay` (`self.WBP_MainMenu`))
  (`self.Reset variable`)
  (`/Game/UI/WBP_GameMenu.SetMultiplicateur` _wbp_gamemenu (`self.CurentMultiplier`))
  (`/Game/UI/WBP_GameMenu.SetScore` _wbp_gamemenu (`KismetMathLibrary.FFloor` (`self.currentScore`)))
  (set `/Game/Blueprint/BP_GameInstance.DidHowToPlayTutorial` true (`/Game/Blueprint/FL_MainFunctionLibrary.GetGameInstanceBP`))
  (`/Game/UI/WBP_MainMenu.ShowUIAfterTuto` (`self.WBP_MainMenu`))
  (`/Game/Blueprint/FL_MainFunctionLibrary.SaveGame`)
  (set `self.isDead` false))

(event `self.ReceiveTick`
  (params (DeltaSeconds :type "Float (single-precision)"))
  (bind _indexcurrentangle (`self.IndexCurrentAngle`))
  (bind _indexcurrentangle_2 (`self.IndexCurrentAngle`))
  (bind _rope (`self.Rope`))
  (bind (_returnvalue_x _returnvalue_y _returnvalue_z) (`KismetMathLibrary.BreakVector` (`SceneComponent.K2_GetComponentLocation` (`self.Mesh`))))
  (bind (_returnvalue_x_2 _returnvalue_y_2 _returnvalue_z_2) (`KismetMathLibrary.BreakVector` (`SceneComponent.K2_GetComponentLocation` (`self.Mesh`))))
  (bind _returnvalue (`KismetMathLibrary.VSize` (`self.vectoAttachActor`)))
  (bind (_returnvalue_x_3 _returnvalue_y_3 _returnvalue_z_3) (`KismetMathLibrary.BreakVector` (`self.K2_GetActorLocation` (`/Game/Blueprint/GameManager/BP_GameManagerMaster.DeadZone` (`self.GameManager`)))))
  (bind (_x _y _z) (`KismetMathLibrary.BreakVector3f` (`self.K2_GetActorLocation` (`self.overlappedAttachPoint`))))
  (bind _returnvalue_2 (`KismetMathLibrary.FFloor` (* (* (`self.speed`) 60.0) DeltaSeconds)))
  (bind _returnvalue_3 (- (`KismetArrayLibrary.Array_Length` (`/Game/Blueprint/BP_GameInstance.YCoordinateCircle` (`self.GameInstance`))) 1))
  (bind _returnvalue_4 (`KismetMathLibrary.SelectInt` _returnvalue_2 (* _returnvalue_2 -1) (`self.rotateClockwise?`)))
  (`|ExecutionSequence`
    (:`then_0`
      (if (`self.isAttached?`)
        (set `self.deltaTimeTick` DeltaSeconds)
        (`SceneComponent.K2_SetWorldLocation` (`self.Mesh`) (`KismetMathLibrary.MakeVector` 0.0 (+ _y (* _returnvalue (`|GetArrayItem` (`/Game/Blueprint/BP_GameInstance.YCoordinateCircle` (`self.GameInstance`)) (`self.IndexCurrentAngle`)))) (+ _z (* (`|GetArrayItem` (`/Game/Blueprint/BP_GameInstance.ZCoordinateCircle` (`self.GameInstance`)) (`self.IndexCurrentAngle`)) _returnvalue))) false false)
        (`SceneComponent.SetWorldScale3D` _rope (`KismetMathLibrary.MakeVector` 1.0 _returnvalue 1.0))
        (`SceneComponent.K2_SetRelativeRotation` _rope (`KismetMathLibrary.MakeRotator` (/ (`self.IndexCurrentAngle`) -50)) false false)
        (`SceneComponent.K2_SetWorldLocation` (`self.Rope`) (`self.K2_GetActorLocation` (`self.overlappedAttachPoint`)) false false)
        (`SceneComponent.K2_AddRelativeRotation` (`self.Skin`) (`KismetMathLibrary.MakeRotator` (* _returnvalue_4 -0.02)) false false)
        (bind _output_get (set `self.IndexCurrentAngle` (+ _indexcurrentangle_2 _returnvalue_4)))
        ;[1 1 1] If clowise turn
        (if (> _indexcurrentangle_2 _returnvalue_3)
          (set `self.IndexCurrentAngle` (- _output_get _returnvalue_3))
          (else
            ;[1 1 1] If anti clockwise turn
            (if (< _indexcurrentangle 0)
              (set `self.IndexCurrentAngle` (+ (- (`KismetArrayLibrary.Array_Length` (`/Game/Blueprint/BP_GameInstance.YCoordinateCircle` (`self.GameInstance`))) 1) _indexcurrentangle)))))))
    (:`then_1`
      ;[0.1647 0.6875 0.4379] MaterialParallax
      (for _array_element (`self.ParalaxBackground`)
        (`MaterialInstanceDynamic.SetVectorParameterValue` _array_element "Location" (`KismetMathLibrary.MakeColor` 0.0 _returnvalue_y _returnvalue_z))))
    (:`then_2`
      ;[1 1 1] Died by zone
      (if (not (`self.firstTouch?`))
        (`|ExecutionSequence`
          (:`then_0`
            (if (< _returnvalue_z_2 _returnvalue_z_3)
              (`self.Death`)))
          (:`then_1`
            (if (not (`self.isDead`))
              (bind _output_get_2 (set `self.CurentMultiplier` (`KismetMathLibrary.FClamp` (/ (- _returnvalue_z_2 _returnvalue_z_3) 2500.0) 1.0 (`self.CurrentMaxMultiplicater`))))
              (`/Game/UI/WBP_GameMenu.SetMultiplicateur` (`self.WBP_GameMenu`) _output_get_2))))))))

(fn `AddScore`
  (params (AmountToAdd :type "Float (double-precision)"))
  (set `self.currentScore` (+ (`self.currentScore`) (* AmountToAdd (`KismetMathLibrary.FFloor` (`self.CurentMultiplier`)))))
  (`/Game/UI/WBP_GameMenu.SetScore` (`self.WBP_GameMenu`) (`KismetMathLibrary.FFloor` (`self.currentScore`))))

(fn `AddStat`
  (params (Stat :type "Float (double-precision)") (Percentage :type Integer))
  (returns (ReturnValue :type "Float (double-precision)"))
  (return (+ Stat (* Stat (/ Percentage 100)))))

(fn `CreateDynamicBackgroundParalax`
  (bind _paralaxbackground (`self.ParalaxBackground`))
  (`|ExecutionSequence`
    (:`then_0`
      (bind _returnvalue (`PrimitiveComponent.CreateDynamicMaterialInstance` (`self.cloud1`) 0 (`PrimitiveComponent.GetMaterial` (`self.cloud1`) 0) "None"))
      (`KismetArrayLibrary.Array_Add` _paralaxbackground _returnvalue)
      (`MaterialInstanceDynamic.SetScalarParameterValue` _returnvalue "PercentageParallax" 0.06))
    (:`then_1`
      (bind _returnvalue_2 (`PrimitiveComponent.CreateDynamicMaterialInstance` (`self.cloud2`) 0 (`PrimitiveComponent.GetMaterial` (`self.cloud2`) 0) "None"))
      (`KismetArrayLibrary.Array_Add` _paralaxbackground _returnvalue_2)
      (`MaterialInstanceDynamic.SetScalarParameterValue` _returnvalue_2 "PercentageParallax" 0.03))
    (:`then_2`
      (bind _returnvalue_3 (`PrimitiveComponent.CreateDynamicMaterialInstance` (`self.cloud3`) 0 (`PrimitiveComponent.GetMaterial` (`self.cloud3`) 0) "None"))
      (`KismetArrayLibrary.Array_Add` _paralaxbackground _returnvalue_3)
      (`MaterialInstanceDynamic.SetScalarParameterValue` _returnvalue_3 "PercentageParallax" 0.01))))

(fn `Disable_EnableInput`
  (params (`Enable?` :type Boolean))
  (bind _returnvalue (`GameplayStatics.GetPlayerController` 0))
  (if `Enable?`
    (`self.EnableInput` _returnvalue)
    (else
      (`self.DisableInput` _returnvalue))))

(fn `RemoveStat`
  (params (Stat :type "Float (double-precision)") (Percentage :type Integer))
  (returns (ReturnValue :type "Float (double-precision)"))
  (return (- Stat (* Stat (/ Percentage 100)))))

(fn `Reset variable`
  (`|ExecutionSequence`
    (:`then_0`
      (set `self.overlappedAttachPoint` null)
      (set `self.firstTouch?` true)
      (set `self.isAttached?` false)
      (set `self.IndexCurrentAngle` 0))
    (:`then_1`
      (set `self.vectoAttachActor` (0.0 0.0 0.0))
      (set `self.deltaTimeTick` 0.0)
      (set `self.CurentMultiplier` 1.0))
    (:`then_2`
      (set `self.currentScore` 0.0)
      (set `self.speed` (`self.baseSpeed`)))))

(fn `ResetPlayer`
  (bind _camera (`self.Camera`))
  (`PrimitiveComponent.SetSimulatePhysics` (`self.Mesh`) false)
  (`SceneComponent.K2_SetWorldLocation` (`self.Mesh`) (0.0 -350.0 1000.0) false false)
  (`SceneComponent.K2_AttachToComponent` _camera (`self.Mesh`) "None" "KeepRelative" "KeepWorld" "KeepWorld" false)
  (`SceneComponent.K2_AttachToComponent` (`self.background`) (`self.Mesh`) "None" "KeepRelative" "KeepWorld" "KeepWorld" false)
  (`SceneComponent.K2_SetRelativeLocation` _camera (-5000.0 0.0 100.0) false false)
  (`SceneComponent.K2_SetRelativeLocation` (`self.background`) (2900.0 0.0 0.0) false false))

(fn `SetPlayerEquipementStat`
  (bind _stats (`/Game/Blueprint/BP_GameInstance.Calculate Equipement Stat` (`self.GameInstance`)))
  (`|ExecutionSequence`
    (:`then_0`
      (bind (_baseaddamountscorepersecond _multiplierdelay _maxmultiplier) (break `/Game/Miscellaneous/DT_Equipement/S_EquipementStat` _stats))
      (set `self.CurrentAddAmountScore` (`self.AddStat` (`self.BaseAddAmountScore`) _baseaddamountscorepersecond)))
    (:`then_1`
      (set `self.CurrentDelayMultipler` (`self.RemoveStat` (`self.BaseDelayMultipler`) _multiplierdelay)))
    (:`then_2`
      (set `self.CurrentMaxMultiplicater` (`self.AddStat` (`self.BaseMaxMultiplier`) _maxmultiplier)))))

(fn `UserConstructionScript`)