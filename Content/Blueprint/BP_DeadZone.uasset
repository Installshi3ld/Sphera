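; BP_DeadZone is an actor that moves along world Z while a game is in progress.
; StartGame and EndGame toggle the movement, which adds Speed every Tick without delta-time scaling, and RestartGame returns it to the position saved at BeginPlay.
; When a BP_AttachPoint stops overlapping its RemoveAttachPoint component, it destroys that attach point if flagged DestroyOnRestart.
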(event `self.ReceiveBeginPlay`
  (set `self.initialPosition` (`self.K2_GetActorLocation`)))

(event `RestartGame`
  (`self.K2_SetActorLocation` (`self.initialPosition`)))

(event `StartGame`
  (set `self.isPlaying` true))

(event `EndGame`
  (set `self.isPlaying` false))

(event `self.ReceiveTick`
  (params (DeltaSeconds :type "Float (single-precision)"))
  (if (`self.isPlaying`)
    (`self.K2_AddActorWorldOffset` (`KismetMathLibrary.MakeVector` 0.0 0.0 (`self.speed`)))))

(event `self.RemoveAttachPoint.OnComponentEndOverlap`
  (params (OverlappedComponent :type "PrimitiveComponent Object Reference") (OtherActor :type "Actor Object Reference") (OtherComp :type "PrimitiveComponent Object Reference") (OtherBodyIndex :type Integer))
  (if (== (`GameplayStatics.GetObjectClass` OtherActor) "/Game/Blueprint/BP_AttachPoint.BP_AttachPoint_C")
    (bind _asbp_attach_point (cast `/Game/Blueprint/BP_AttachPoint` OtherActor))
    (if (`/Game/Blueprint/BP_AttachPoint.destroyOnRestart?` _asbp_attach_point)
      (`self.K2_DestroyActor` OtherActor))))

(fn `UserConstructionScript`)