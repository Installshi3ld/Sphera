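; BP_MultiplicaterOverlap is a drop-ball game trigger actor that applies a score multiplier to balls that overlap it.
; At BeginPlay it passes its multiplier value to its WBP_MultiplicaterDropBall widget and caches the BP_PlayerDropBall found in the level.
; On overlap with a BP_Ball, it sets that ball's multiply score, then notifies the player through MultiplicaterOverlapEvent.
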(event `self.ReceiveBeginPlay`
  (bind _aswbp_multiplicater_drop_ball (cast `/Game/UI/DropBall/WBP_MultiplicaterDropBall` (`WidgetComponent.GetWidget` (`self.Widget`))))
  (`/Game/UI/DropBall/WBP_MultiplicaterDropBall.SetMultiplicaterValue` _aswbp_multiplicater_drop_ball (`self.multiplicaterValue`))
  (bind _returnvalue (`GameplayStatics.GetActorOfClass` "/Game/Blueprint/DropBall/BP_PlayerDropBall.BP_PlayerDropBall_C"))
  (set `self.PlayerPawn` _returnvalue))

(event `self.ReceiveActorBeginOverlap`
  (params (OtherActor :type "Actor Object Reference"))
  (bind _asbp_ball (cast `/Game/Blueprint/DropBall/BP_Ball` OtherActor))
  (`/Game/Blueprint/DropBall/BP_Ball.SetMultiplyScore` _asbp_ball (`self.multiplicaterValue`))
  (`/Game/Blueprint/DropBall/BP_PlayerDropBall.MultiplicaterOverlapEvent` (`self.PlayerPawn`) _asbp_ball))

(fn `UserConstructionScript`)