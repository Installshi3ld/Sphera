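; Game manager that procedurally spawns an endless chain of BP_AttachPoint actors ahead of the player along the Y axis.
; After a brief BeginPlay delay caches the player pawn, Tick watches its mesh cross each Y threshold.
; Each crossing spawns a point one fixed Y step beyond the last, with a random Z drift biased downward.
; RestartGame resets the spawn tracking and destroys attach points flagged DestroyOnRestart.
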(event `RestartGame`
  (`self.ResetVariable`)
  (bind _outactors (`GameplayStatics.GetAllActorsOfClass` "/Game/Blueprint/BP_AttachPoint.BP_AttachPoint_C"))
  (for _array_element _outactors
    (if (`/Game/Blueprint/BP_AttachPoint.destroyOnRestart?` _array_element)
      (`self.K2_DestroyActor` _array_element))))

(event `self.ReceiveTick`
  (params (DeltaSeconds :type "Float (single-precision)"))
  (bind (_x _y _z) (`KismetMathLibrary.BreakVector3f` (`self.lastSpawnedAttachPointCoordinate`)))
  (bind _returnvalue (`KismetMathLibrary.MakeVector` 0.0 (+ (`self.spawnEveryY`) _y) (+ _z (`KismetMathLibrary.RandomFloatInRange` -700.0 250.0))))
  (if (`self.readyToPlay`)
    (if (> (`.Y` (`KismetMathLibrary.BreakVector3f` (`SceneComponent.K2_GetComponentLocation` (`/Game/Blueprint/BP_Player.Mesh` (`self.playerControlledPawn`))))) (`self.nextSpawningCoordinateY`))
      (set `self.nextSpawningCoordinateY` (+ (`self.nextSpawningCoordinateY`) (`self.spawnEveryY`)))
      (`|SpawnActorFromClass` "/Game/Blueprint/BP_AttachPoint.BP_AttachPoint_C" (`KismetMathLibrary.MakeTransform` _returnvalue) "Undefined" "OverrideRootScale" null true null)
      (set `self.lastSpawnedAttachPointCoordinate` _returnvalue))))

(event `self.ReceiveBeginPlay`
  (`KismetSystemLibrary.Delay` 0.001)
  (set `self.readyToPlay` true)
  (bind _asbp_player (cast `/Game/Blueprint/BP_Player` (`Controller.K2_GetPawn` (`GameplayStatics.GetPlayerController` 0))))
  (set `self.playerControlledPawn` _asbp_player))

(fn `ResetVariable`
  (set `self.lastSpawnedAttachPointCoordinate` (0.0 1600.0 430.0))
  (set `self.nextSpawningCoordinateY` 0.0))

(fn `UserConstructionScript`)