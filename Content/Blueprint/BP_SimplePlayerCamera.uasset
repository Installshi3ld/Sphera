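; Player camera Blueprint that runs a ball-drop race, spawning up to five balls from the GameInstance inventory.
; BeginPlay rerolls random Y positions to keep balls spaced apart, copying each item's mesh, material and score.
; A touch or click enables physics ball by ball on a timer and starts a periodic upward nudge for unfinished balls.
; Multiplier overlaps record finishers and call FinishLevel, which is empty.
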(event `self.ReceiveBeginPlay`
  (bind _coordinatevalid_ (`self.coordinateValid?`))
  (bind _tmprandomyfloat (`self.tmpRandomYFloat`))
  (bind _tmprandomyfloat_2 (`self.tmpRandomYFloat`))
  (bind (_output_mesh _output_material _output_score) (break `/Game/Miscellaneous/S_BallData` (`|GetArrayItem` (`/Game/Blueprint/BP_GameInstance.BallInventory` (`self.GameInstance`)) (`KismetArrayLibrary.Array_Length` (`self.SpawnedBalls`)))))
  (`Controller.Possess` (`GameplayStatics.GetPlayerController` 0) null)
  (set `self.GameInstance` (cast `/Game/Blueprint/BP_GameInstance` (`GameplayStatics.GetGameInstance`) :!pure true))
  (`WidgetLayoutLibrary.RemoveAllWidgets`)
  (for _ (range (+ (`KismetMathLibrary.Clamp` (- (`KismetArrayLibrary.Array_Length` (`/Game/Blueprint/BP_GameInstance.BallInventory` (`self.GameInstance`))) 1) 0 4) 1))
    ;[1 1 1] Get random pos for ball
    (set `self.tmpRandomYFloat` (`KismetMathLibrary.RandomFloatInRange` -350.0 350.0) :!label _label)
    (for (_array_element _array_index) (`self.YCoordinateSpawnReserved`)
      (if (and (> _tmprandomyfloat (- _array_element 55.0)) (< _tmprandomyfloat (+ _array_element 55.0)))
        (`KismetArrayLibrary.Array_Set` _coordinatevalid_ _array_index false true)
        (else
          (`KismetArrayLibrary.Array_Set` _coordinatevalid_ _array_index true true))))
    (if (`KismetArrayLibrary.Array_Contains` (`self.coordinateValid?`))
      (goto _label)
      (else
        (`KismetArrayLibrary.Array_Add` (`self.YCoordinateSpawnReserved`) _tmprandomyfloat_2)
        (bind _returnvalue (`|SpawnActorFromClass` "/Game/Blueprint/BP_Ball.BP_Ball_C" (`KismetMathLibrary.MakeTransform` (`KismetMathLibrary.MakeVector` 0.0 _tmprandomyfloat_2 800.0)) "Undefined" "OverrideRootScale" null null))
        (bind _mesh (`/Game/Blueprint/BP_Ball.Mesh` _returnvalue))
        ;[1 1 1] Set ball skin, mesh and
        (`StaticMeshComponent.SetStaticMesh` _mesh _output_mesh)
        (`PrimitiveComponent.SetMaterial` _mesh 0 _output_material)
        (set `/Game/Blueprint/BP_Ball.Score` _output_score _returnvalue)
        (`KismetArrayLibrary.Array_Add` (`self.SpawnedBalls`) _returnvalue))))
  (set `self.CanReleaseBalls` true))

(event `FinishLevel`)

(event `MultiplicaterOverlapEvent`
  (params (BallOverlapped :type "/Game/Blueprint/BP_Ball Object Reference"))
  (bind _returnvalue (`KismetArrayLibrary.Array_Add` (`self.ballEndRace`) BallOverlapped))
  (if (>= _returnvalue (- (`KismetArrayLibrary.Array_Length` (`self.SpawnedBalls`)) 1))
    (`self.FinishLevel`)))

(event `CheckIfBallIsStuck`
  ;[1 1 1] CheckIfBallStuck
  (`KismetSystemLibrary.K2_SetTimerDelegate` (delegate `CheckIfBallIsStuck`) 10.0 true)
  (if (`self.AvoidFirstTeleportBallStuck`)
    (for _array_element (`self.SpawnedBalls`)
      (if (not (`KismetArrayLibrary.Array_Contains` (`self.ballEndRace`) _array_element))
        (`SceneComponent.K2_AddWorldOffset` (`/Game/Blueprint/BP_Ball.Mesh` _array_element) (0.0 0.0 100.0) false false)))
    (else
      (set `self.AvoidFirstTeleportBallStuck` true))))

(event `InputTouch`
  (params (Location :type "Vector Structure") (FingerIndex :type "ETouchIndex Enum"))
  ;[1 1 1] InputTouch
  (:`Pressed`
    (if (`self.CanReleaseBalls`) :!label _label_2
      (if (not (`self.ballReleased`))
        (`self.ReleaseBall`)
        (`self.CheckIfBallIsStuck`)
        (set `self.ballReleased` true)))))

(event `Key|LeftMouseButton`
  (params (Key :type "Key Structure"))
  ;[1 1 1] InputTouch
  (:`Pressed`
    (goto _label_2)))

(event `ReleaseBall`
  (bind _tmpreleasedballindex (`self.tmpReleasedBallIndex`))
  (bind _output (`|GetArrayItem` (`self.SpawnedBalls`) _tmpreleasedballindex))
  ;[1 1 1] ReleaseBAll
  (bind _returnvalue (`KismetSystemLibrary.K2_SetTimerDelegate` (delegate `ReleaseBall`) 0.2))
  (`/Engine/EditorBlueprintResources/StandardMacros.IncrementInt` _tmpreleasedballindex
    (:`  `
      (`/Engine/EditorBlueprintResources/StandardMacros.IsValid` _output
        (:`Is Valid`
          (`PrimitiveComponent.SetSimulatePhysics` (`/Game/Blueprint/BP_Ball.Mesh` _output) true))
        (:`Is Not Valid`
          (`KismetSystemLibrary.K2_ClearAndInvalidateTimerHandle` _returnvalue))))))

(fn `Get Random Position for Ball`
  (params (`ForAllBall?` :type Boolean))
  (bind _tmprandomyfloat (`self.tmpRandomYFloat`))
  (bind _coordinatevalid_ (`self.coordinateValid?`))
  (bind _tmprandomyfloat_2 (`self.tmpRandomYFloat`))
  (bind _returnvalue (`KismetArrayLibrary.Array_Length` (`self.SpawnedBalls`)))
  (`KismetArrayLibrary.Array_Clear` (`self.coordinateValid?`))
  (`KismetArrayLibrary.Array_Clear` (`self.YCoordinateSpawnReserved`))
  (if `ForAllBall?`
    (for _ (range (+ (`KismetMathLibrary.SelectInt` (- _returnvalue 1) (- (- _returnvalue (`KismetArrayLibrary.Array_Length` (`self.ballEndRace`))) 1) `ForAllBall?`) 1))
      (set `self.tmpRandomYFloat` (`KismetMathLibrary.RandomFloatInRange` -350.0 350.0) :!label _label)
      (for (_array_element _array_index) (`self.YCoordinateSpawnReserved`)
        (if (and (> _tmprandomyfloat_2 (- _array_element 55.0)) (< _tmprandomyfloat_2 (+ _array_element 55.0)))
          (`KismetArrayLibrary.Array_Set` _coordinatevalid_ _array_index false true)
          (else
            (`KismetArrayLibrary.Array_Set` _coordinatevalid_ _array_index true true))))
      (if (`KismetArrayLibrary.Array_Contains` (`self.coordinateValid?`))
        (goto _label)
        (else
          (`KismetArrayLibrary.Array_Add` (`self.YCoordinateSpawnReserved`) _tmprandomyfloat)
          (bind _returnvalue_2 (`|SpawnActorFromClass` "/Game/Blueprint/BP_Ball.BP_Ball_C" (`KismetMathLibrary.MakeTransform` (`KismetMathLibrary.MakeVector` 0.0 _tmprandomyfloat 800.0)) "Undefined" "OverrideRootScale" null null))
          (`KismetArrayLibrary.Array_Add` (`self.SpawnedBalls`) _returnvalue_2))))
    (set `self.CanReleaseBalls` true)
    (else
      (goto _label))))

(fn `UserConstructionScript`)