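; Player controller that creates and holds the game's overlay widgets and handles possessing a pawn.
; BeginPlay uses a sequence to create, store and add to the viewport the spin wheel, item description, ad loading, slot add-item and difficulty selection widgets.
; PossessEntity switches input to Game and UI before possessing the given pawn.
; Getters expose the spin wheel and item description widgets; tutorial screen creation is present but never runs.
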(event `self.ReceiveBeginPlay`
  (`|ExecutionSequence`
    (:`then_0`
      (bind _returnvalue (`|CreateWidget` "/Game/UI/SkinWheel/WBP_SpinWheel.WBP_SpinWheel_C"))
      (set `self.WBP_SpinWheel` _returnvalue)
      (`UserWidget.AddToViewport` _returnvalue 0)
      (bind _returnvalue_2 (`|CreateWidget` "/Game/UI/WBP_ItemDescriptionWIndow.WBP_ItemDescriptionWIndow_C"))
      (`UserWidget.AddToViewport` _returnvalue_2 0)
      (set `self.WBP_itemDescription` _returnvalue_2))
    (:`then_1`
      (bind _returnvalue_3 (`|CreateWidget` "/Game/UI/WBP_AdLoadingScreen.WBP_AdLoadingScreen_C"))
      (`UserWidget.AddToViewport` _returnvalue_3 0)
      (set `self.WBP_AdLoadingScreen` _returnvalue_3)
      (bind _returnvalue_4 (`|CreateWidget` "/Game/UI/Inventory/WBP_SlotAddItem.WBP_SlotAddItem_C"))
      (`UserWidget.AddToViewport` _returnvalue_4 0)
      (set `self.WBP_SlotAddItem` _returnvalue_4))
    (:`then_2`
      (bind _returnvalue_5 (`|CreateWidget` "/Game/UI/SelectDifficulty/WBP_SelectDifficulty_RaiseUp.WBP_SelectDifficulty_RaiseUp_C"))
      (`UserWidget.AddToViewport` _returnvalue_5 0)
      (set `self.WBP_SelectDifficulty_RaiseUp` _returnvalue_5))))

(event `PossessEntity`
  (params (InPawn :type "Pawn Object Reference"))
  (`WidgetBlueprintLibrary.SetInputMode_GameAndUIEx` self null "DoNotLock" false)
  (`self.Possess` InPawn))

(fn `GetWBP_ItemDescription`
  (returns (WBP_itemDescription :type "/Game/UI/WBP_ItemDescriptionWIndow Object Reference"))
  (return (`self.WBP_itemDescription`)))

(fn `GetWBP_SpinWheel`
  (returns (WBP_SpinWheel :type "/Game/UI/SkinWheel/WBP_SpinWheel Object Reference"))
  (return (`self.WBP_SpinWheel`)))

(fn `UserConstructionScript`)