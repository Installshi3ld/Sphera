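; BP_GameManagerMaster is the master game manager that handles starting and restarting a run.
; On BeginPlay, after a tiny delay, it flags readiness, caches the controlled BP_Player and spawns a BP_DeadZone at its own location.
; StartGame forwards to the dead zone, while RestartGame resets attach-point spawn coordinates, destroys attach points flagged DestroyOnRestart and restarts the dead zone.
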(event `self.ReceiveBeginPlay`
  (`KismetSystemLibrary.Delay` 0.001)
  (set `self.readyToPlay` true)
  (bind _asbp_player (cast `/Game/Blueprint/BP_Player` (`Controller.K2_GetPawn` (`GameplayStatics.GetPlayerController` 0))))
  (set `self.playerControlledPawn` _asbp_player)
  (bind _returnvalue (`|SpawnActorFromClass` "/Game/Blueprint/BP_DeadZone.BP_DeadZone_C" (`KismetMathLibrary.MakeTransform` (`self.K2_GetActorLocation` self)) "Undefined" "OverrideRootScale" null null))
  (set `self.DeadZone` _returnvalue))

(event `RestartGame`
  (`self.ResetVariable`)
  (bind _outactors (`GameplayStatics.GetAllActorsOfClass` "/Game/Blueprint/BP_AttachPoint.BP_AttachPoint_C"))
  (for _array_element _outactors
    (if (`/Game/Blueprint/BP_AttachPoint.destroyOnRestart?` _array_element)
      (`self.K2_DestroyActor` _array_element)))
  (`/Game/Blueprint/BP_DeadZone.RestartGame` (`self.DeadZone`)))

(event `StartGame`
  (`/Game/Blueprint/BP_DeadZone.StartGame` (`self.DeadZone`)))

(fn `ResetVariable`
  (set `self.lastSpawnedAttachPointCoordinate` (0.0 0.0 2300.0))
  (set `self.nextSpawningCoordinateZ` 0.0))

(fn `UserConstructionScript`)