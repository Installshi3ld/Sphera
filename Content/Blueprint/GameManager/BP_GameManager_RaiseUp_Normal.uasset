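; Game manager for the normal RaiseUp mode that endlessly spawns BP_AttachPoint actors as the player pawn rises.
; Once ready to play, Tick compares the pawn mesh's height to a threshold that advances by a fixed Z step.
; Each crossing spawns a row one step above the last: a randomly jittered center point and two lower points far out on either side along Y.
; The stored last coordinate then advances for the next row.
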(event `self.ReceiveTick`
  (params (DeltaSeconds :type "Float (single-precision)"))
  (bind _returnvalue (+ (`.Z` (`KismetMathLibrary.BreakVector3f` (`self.lastSpawnedAttachPointCoordinate`))) (`self.spawnEveryZ`)))
  (bind _returnvalue_2 (`KismetMathLibrary.MakeVector` 0.0 (`KismetMathLibrary.RandomFloatInRange` -100.0 100.0) _returnvalue))
  (bind _returnvalue_3 (- _returnvalue 450.0))
  (if (`self.readyToPlay`)
    (if (> (`.Z` (`KismetMathLibrary.BreakVector3f` (`SceneComponent.K2_GetComponentLocation` (`/Game/Blueprint/BP_Player.Mesh` (`self.playerControlledPawn`))))) (`self.nextSpawningCoordinateZ`))
      (set `self.nextSpawningCoordinateZ` (+ (`self.nextSpawningCoordinateZ`) (`self.spawnEveryZ`)))
      (`|SpawnActorFromClass` "/Game/Blueprint/BP_AttachPoint.BP_AttachPoint_C" (`KismetMathLibrary.MakeTransform` _returnvalue_2) "Undefined" "OverrideRootScale" null true null)
      (`|SpawnActorFromClass` "/Game/Blueprint/BP_AttachPoint.BP_AttachPoint_C" (`KismetMathLibrary.MakeTransform` (`KismetMathLibrary.MakeVector` 0.0 (`KismetMathLibrary.RandomFloatInRange` 1000.0 1100.0) _returnvalue_3)) "Undefined" "OverrideRootScale" null true null)
      (`|SpawnActorFromClass` "/Game/Blueprint/BP_AttachPoint.BP_AttachPoint_C" (`KismetMathLibrary.MakeTransform` (`KismetMathLibrary.MakeVector` 0.0 (`KismetMathLibrary.RandomFloatInRange` -1000.0 -1100.0) _returnvalue_3)) "Undefined" "OverrideRootScale" null true null)
      (set `self.lastSpawnedAttachPointCoordinate` _returnvalue_2))))

(fn `UserConstructionScript`)