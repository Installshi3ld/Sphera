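; Game manager for the hard RaiseUp mode that procedurally spawns the level as the player climbs along Z.
; On Tick, once ready to play, each time the pawn's mesh passes the next height threshold it spawns a near-center attach point and a lower side one.
; A FlipFlop alternates the side point between left and right.
; Each step also advances the last spawn coordinate and has a small random chance to spawn a laser near the center.
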(event `self.ReceiveTick`
  (params (DeltaSeconds :type "Float (single-precision)"))
  (bind _returnvalue (`KismetMathLibrary.RandomFloatInRange` -100.0 100.0))
  (bind _returnvalue_2 (+ (`.Z` (`KismetMathLibrary.BreakVector3f` (`self.lastSpawnedAttachPointCoordinate`))) (`self.spawnEveryZ`)))
  (bind _returnvalue_3 (`KismetMathLibrary.MakeVector` 0.0 _returnvalue _returnvalue_2))
  (bind _returnvalue_4 (- _returnvalue_2 475.0))
  (if (`self.readyToPlay`)
    (if (> (`.Z` (`KismetMathLibrary.BreakVector3f` (`SceneComponent.K2_GetComponentLocation` (`/Game/Blueprint/BP_Player.Mesh` (`self.playerControlledPawn`))))) (`self.nextSpawningCoordinateZ`))
      (set `self.nextSpawningCoordinateZ` (+ (`self.nextSpawningCoordinateZ`) (`self.spawnEveryZ`)))
      (`|SpawnActorFromClass` "/Game/Blueprint/BP_AttachPoint.BP_AttachPoint_C" (`KismetMathLibrary.MakeTransform` _returnvalue_3) "Undefined" "OverrideRootScale" null true null)
      (`|SpawnActorFromClass` "/Game/Blueprint/BP_AttachPoint.BP_AttachPoint_C" (`KismetMathLibrary.MakeTransform` (`KismetMathLibrary.MakeVector` 0.0 (* (`KismetMathLibrary.RandomFloatInRange` 1000.0 1100.0) (`KismetMathLibrary.SelectFloat` 1.0 -1.0 (`self.spawnLeft?`))) _returnvalue_4)) "Undefined" "OverrideRootScale" null true null)
      (`|ExecutionSequence`
        (:`then_0`
          (set `self.lastSpawnedAttachPointCoordinate` _returnvalue_3)
          (`/Engine/EditorBlueprintResources/StandardMacros.FlipFlop`
            (:`A`
              (set `self.spawnLeft?` true))
            (:`B`
              (set `self.spawnLeft?` false))))
        (:`then_1`
          (if (< (`KismetMathLibrary.RandomInteger` 100) 10)
            (`|SpawnActorFromClass` "/Game/Blueprint/BP_Laser.BP_Laser_C" (`KismetMathLibrary.MakeTransform` (`KismetMathLibrary.MakeVector` 0.0 _returnvalue _returnvalue_4)) "Undefined" "OverrideRootScale" null null)))))))

(fn `UserConstructionScript`)