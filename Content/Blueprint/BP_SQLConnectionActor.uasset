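; An actor for SQL database access meant to register a new player ID, but its logic is disconnected, so only TryCreateIDinDB does anything: it sets a flag.
; The unwired chains open a connection using GameInstance settings and a hardcoded password, then insert a PlayerInfo row.
; A RequestSent queue would route query callbacks to use the row count as PlayerID, set a default username and save.
; A stray SpheraInfo insert is also unwired.
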(event `self.ReceiveBeginPlay`)

(event `Try Create ID in DB`
  (set `self.TryCreatePlayerID` true))

(event `Key|Android_Menu`
  (params (Key :type "Key Structure")))

(event `self.OnConnectionStateChanged`
  (params (ConnectionStatus :type Boolean) (ConnectionID :type Integer) (ErrorMessage :type String)))

(event `self.OnQueryUpdateStatusChanged`
  (params (IsSuccessful :type Boolean) (ErrorMessage :type String)))

(event `CreatePlayerID`)

(event `self.OnQuerySelectStatusChanged`
  (params (IsSuccessful :type Boolean) (ErrorMessage :type String) (ResultByColumn :type "Array of MySQLDataTable Structure (by ref)") (ResultByRow :type "Array of MySQLDataRow Structure (by ref)")))

(fn `UserConstructionScript`)