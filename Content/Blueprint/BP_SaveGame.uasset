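; BP_SaveGame stores the item inventory and equipped runes and rebuilds them on load.
; Items flatten into SBaseInventorySave structs holding class, shared fields and extras for equipment, skins and spheras; loading constructs objects from the class and restores those fields.
; Equipped runes are saved as inventory indices, resolved on load by scanning the inventory, with empty entries inserted for -1 slots.
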(fn `LoadEquipedRune`
  (params (Inventory :type "Array of /Game/ItemData/DA_BaseInventoryObject Object Reference"))
  (returns (EquipedRune :type "Array of /Game/ItemData/Equipement/DA_Equipement Object Reference"))
  (locals (tmpEquipedRune :type "Array of /Game/ItemData/Equipement/DA_Equipement Object Reference"))
  (for (_ _array_index) Inventory
    (for _index (range (`KismetArrayLibrary.Array_Length` (`self.equipedRune`)))
      (bind _output (`|GetArrayItem` (`self.equipedRune`) _index))
      (if (== _array_index _output)
        (`KismetArrayLibrary.Array_Add` (`local.tmpEquipedRune`) (cast `/Game/ItemData/Equipement/DA_Equipement` (`|GetArrayItem` (`local.Inventory`) _output) :!pure true)))))
  ;[1 1 1] CheckEmptySlot and add empty rune
  (for (_array_element _array_index_2) (`self.equipedRune`)
    (if (== _array_element -1)
      (`KismetArrayLibrary.Array_Insert` (`local.tmpEquipedRune`) null _array_index_2)))
  (return (`local.tmpEquipedRune`)))

(fn `LoadInventory`
  (returns (ItemInventory :type "Array of /Game/ItemData/DA_BaseInventoryObject Object Reference"))
  (locals (tmpInventory :type "Array of /Game/ItemData/DA_BaseInventoryObject Object Reference"))
  (for _array_element (`self.itemInventory`)
    (bind (_class _name _amount _image _description _rarity _runeemplacement _isunlock _spherascore _spheraskeletalmesh) (break `/Game/Miscellaneous/StructSave/S_BaseInventorySave` _array_element))
    (bind _returnvalue (`|GenericCreateObject` _class))
    (`|ExecutionSequence`
      (:`then_0`
        (`/Game/ItemData/DA_BaseInventoryObject.SetName` _returnvalue _name))
      (:`then_1`
        (`/Game/ItemData/DA_BaseInventoryObject.SetAmount` _returnvalue _amount))
      (:`then_2`
        (`/Game/ItemData/DA_BaseInventoryObject.SetImage` _returnvalue _image))
      (:`then_3`
        (`/Game/ItemData/DA_BaseInventoryObject.SetDescription` _returnvalue _description))
      (:`then_4`
        (`/Game/ItemData/DA_BaseInventoryObject.SetRarity` _returnvalue _rarity))
      (:`then_5`
        (bind _asda_equipement (cast `/Game/ItemData/Equipement/DA_Equipement` _returnvalue))
        (`/Game/ItemData/Equipement/DA_Equipement.SetRuneEmplacement` _asda_equipement _runeemplacement))
      (:`then_6`
        (bind _asda_skin (cast `/Game/ItemData/Skin/DA_Skin` _returnvalue))
        (`/Game/ItemData/Skin/DA_Skin.SetIsUnlocked` _asda_skin _isunlock))
      (:`then_7`
        (bind _asda_sphera (cast `/Game/ItemData/DA_Sphera` _returnvalue))
        (`/Game/ItemData/DA_Sphera.SetScore` _asda_sphera _spherascore))
      (:`then_8`
        (bind _asda_sphera_2 (cast `/Game/ItemData/DA_Sphera` _returnvalue))
        (`/Game/ItemData/DA_Sphera.SetSkeletalMesh` _asda_sphera_2 _spheraskeletalmesh))
      (:`then_9`
        (`KismetArrayLibrary.Array_Add` (`local.tmpInventory`) _returnvalue))))
  (return (`local.tmpInventory`)))

(fn `SaveEquipedRune`
  (params (Inventory :type "Array of /Game/ItemData/DA_BaseInventoryObject Object Reference") (equipedRune :type "Array of /Game/ItemData/Equipement/DA_Equipement Object Reference"))
  (`KismetArrayLibrary.Array_Clear` (`self.equipedRune`))
  (for _array_element equipedRune
    (`KismetArrayLibrary.Array_Add` (`self.equipedRune`) (`KismetArrayLibrary.Array_Find` Inventory _array_element))))

(fn `SaveInventory`
  (params (ItemInventory :type "Array of /Game/ItemData/DA_BaseInventoryObject Object Reference"))
  (bind _iteminventory (`self.itemInventory`))
  (`KismetArrayLibrary.Array_Clear` (`self.itemInventory`))
  (for _array_element ItemInventory
    (bind _asda_equipement (cast `/Game/ItemData/Equipement/DA_Equipement` _array_element)
      (:`then`
        (bind _returnvalue (`GameplayStatics.GetObjectClass` _array_element))
        (bind _name (`/Game/ItemData/DA_BaseInventoryObject.GetName` _array_element))
        (bind _amount (`/Game/ItemData/DA_BaseInventoryObject.GetAmount` _array_element))
        (bind _image (`/Game/ItemData/DA_BaseInventoryObject.GetImage` _array_element))
        (bind _description (`/Game/ItemData/DA_BaseInventoryObject.GetDescription` _array_element))
        (bind _rarity (`/Game/ItemData/DA_BaseInventoryObject.GetRarity` _array_element))
        (`KismetArrayLibrary.Array_Add` _iteminventory (make `/Game/Miscellaneous/StructSave/S_BaseInventorySave` _returnvalue _name _amount _image _description _rarity (`/Game/ItemData/Equipement/DA_Equipement.GetRuneEmplacment` _asda_equipement))))
      (:`CastFailed`
        (bind _asda_skin (cast `/Game/ItemData/Skin/DA_Skin` _array_element)
          (:`then`
            (`KismetArrayLibrary.Array_Add` _iteminventory (make `/Game/Miscellaneous/StructSave/S_BaseInventorySave` _returnvalue _name _amount _image _description _rarity 0 (`/Game/ItemData/Skin/DA_Skin.GetIsUnlocked` _asda_skin))))
          (:`CastFailed`
            (bind _asda_sphera (cast `/Game/ItemData/DA_Sphera` _array_element)
              (:`then`
                (`KismetArrayLibrary.Array_Add` _iteminventory (make `/Game/Miscellaneous/StructSave/S_BaseInventorySave` _returnvalue _name _amount _image _description _rarity 0 false (`/Game/ItemData/DA_Sphera.Score` _asda_sphera) (`/Game/ItemData/DA_Sphera.SkeletalMesh` _asda_sphera))))
              (:`CastFailed`
                (`KismetArrayLibrary.Array_Add` _iteminventory (make `/Game/Miscellaneous/StructSave/S_BaseInventorySave` _returnvalue _name _amount _image _description _rarity))))))))))