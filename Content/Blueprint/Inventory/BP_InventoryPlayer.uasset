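; BP_InventoryPlayer is the player pawn for the inventory screen, possessed by player controller 0 on BeginPlay.
; It sets the camera's orthographic width from the viewport aspect ratio, keeping a constant vertical view extent as screen shape varies.
; It then creates the WBP_MainInventory widget, adds it to the viewport, shows the mouse cursor and switches input to UI only.
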(event `self.ReceiveBeginPlay`
  (bind _returnvalue (`GameplayStatics.GetPlayerController` 0))
  (bind (_returnvalue_x _returnvalue_y) (`KismetMathLibrary.BreakVector2D` (`WidgetLayoutLibrary.GetViewportSize`)))
  (`CameraComponent.SetOrthoWidth` (`self.Camera`) (* (/ _returnvalue_x _returnvalue_y) 1920.0))
  (`Controller.Possess` _returnvalue self)
  (bind _returnvalue_2 (`|CreateWidget` "/Game/UI/Inventory/WBP_MainInventory.WBP_MainInventory_C" _returnvalue))
  (`UserWidget.AddToViewport` _returnvalue_2 0)
  (set `PlayerController.bShowMouseCursor` true _returnvalue)
  (`WidgetBlueprintLibrary.SetInputMode_UIOnlyEx` (`GameplayStatics.GetPlayerController` 0) null))

(fn `UserConstructionScript`)